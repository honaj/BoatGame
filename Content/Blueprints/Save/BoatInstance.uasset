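; Game instance for the boat game that saves and restores world state through a MainSave object in slot "Save1".
; Init creates a fresh save object, which separate functions fill with player, boat, buoyant actor, sky time and cloud data.
; Only the player, world and cloud saves write to disk.
; LoadGame repositions player and boat, scrubs the sky timeline and spawns saved clouds, but never restores buoyant actors.
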(event `self.ReceiveInit`
  (bind _returnvalue (`GameplayStatics.CreateSaveGameObject` "/Game/Blueprints/Save/MainSave.MainSave_C"))
  (set `self.PlayerSave` _returnvalue))

(fn `LoadGame`
  (bind _returnvalue (`GameplayStatics.DoesSaveGameExist` "Save1"))
  (if _returnvalue
    (bind _returnvalue_2 (`GameplayStatics.LoadGameFromSlot` "Save1"))
    (bind _asmain_save (cast `/Game/Blueprints/Save/MainSave` _returnvalue_2))
    (`|ExecutionSequence`
      (:`then_0`
        ;[1 1 1] Load player
        (bind _asplayer (cast `/Game/Blueprints/Player/Player` (`GameplayStatics.GetPlayerCharacter` 0)))
        (`Actor.K2_SetActorLocation` _asplayer (`/Game/Blueprints/Save/MainSave.PlayerLocation` _asmain_save) false)
        (`SceneComponent.K2_SetWorldRotation` (`Character.CapsuleComponent` _asplayer) (`/Game/Blueprints/Save/MainSave.PlayerCapsuleRotation` _asmain_save) false)
        (`SceneComponent.K2_SetWorldRotation` (`/Game/Blueprints/Player/Player.Camera` _asplayer) (`/Game/Blueprints/Save/MainSave.PlayerCameraRotation` _asmain_save) false))
      (:`then_1`
        ;[1 1 1] Load boat
        (bind _outactors (`GameplayStatics.GetAllActorsOfClass` "/Game/Blueprints/Boat/BP_Boat.BP_Boat_C"))
        (bind _item (`KismetArrayLibrary.Array_Get` _outactors))
        (`/Engine/EditorBlueprintResources/StandardMacros.IsValid` _item
          (:`Is Valid`
            (bind (_boatstruct_location _boatstruct_rotation) (break `/Game/Blueprints/Save/BoatStruct` (`/Game/Blueprints/Save/MainSave.BoatStruct` _asmain_save)))
            (`Actor.K2_SetActorLocationAndRotation` _item _boatstruct_location _boatstruct_rotation false))))
      (:`then_2`
        (bind _outactors_2 (`GameplayStatics.GetAllActorsOfClass` "/Game/Blueprints/World/Sky/SkyControl.SkyControl_C"))
        (bind _worldstruct_time (break `/Game/Blueprints/Save/WorldStruct` (`/Game/Blueprints/Save/MainSave.WorldStruct` _asmain_save)))
        (`TimelineComponent.SetPlaybackPosition` (`/Game/Blueprints/World/Sky/SkyControl.SkyTime` (`KismetArrayLibrary.Array_Get` _outactors_2)) _worldstruct_time false true))
      (:`then_3`
        (for _array_element (`/Game/Blueprints/Save/MainSave.CloudTransforms` _asmain_save)
          (`|SpawnActorFromClass` "/Game/Blueprints/World/Cloud.Cloud_C" _array_element true))))))

(fn `SaveBoat`
  (bind _asmain_save (cast `/Game/Blueprints/Save/MainSave` (`self.PlayerSave`)))
  (bind _outactors (`GameplayStatics.GetAllActorsOfClass` "/Game/Blueprints/Boat/BP_Boat.BP_Boat_C"))
  (bind _item (`KismetArrayLibrary.Array_Get` _outactors))
  (set `/Game/Blueprints/Save/MainSave.BoatStruct` (make `/Game/Blueprints/Save/BoatStruct` (`SceneComponent.K2_GetComponentLocation` (`/Game/Blueprints/Boat/BP_Boat.StaticMesh` _item)) (`Actor.K2_GetActorRotation` _item)) _asmain_save))

(fn `SaveBuoyantActors`
  (bind _outactors (`GameplayStatics.GetAllActorsOfClass` "/Game/Blueprints/BP_BuoyantActor.BP_BuoyantActor_C"))
  (for _array_element _outactors
    (bind _asmain_save (cast `/Game/Blueprints/Save/MainSave` (`self.PlayerSave`)))
    (`KismetArrayLibrary.Array_Add` (`/Game/Blueprints/Save/MainSave.BuoyantActorsLocations` _asmain_save) (`SceneComponent.K2_GetComponentLocation` (`/Game/Blueprints/BP_BuoyantActor.BuoyancyForce` _array_element)))))

(fn `SaveClouds`
  (bind _asmain_save (cast `/Game/Blueprints/Save/MainSave` (`self.PlayerSave`)))
  (bind _outactors (`GameplayStatics.GetAllActorsOfClass` "/Game/Blueprints/World/Cloud.Cloud_C"))
  (for _array_element _outactors
    (`KismetArrayLibrary.Array_Add` (`/Game/Blueprints/Save/MainSave.CloudTransforms` _asmain_save) (`Actor.GetTransform` _array_element)))
  (`GameplayStatics.SaveGameToSlot` _asmain_save "Save1")
  (`KismetSystemLibrary.PrintString` "Hello"))

(fn `SavePlayer`
  (bind _returnvalue (`GameplayStatics.GetPlayerCharacter` 0))
  (bind _asmain_save (cast `/Game/Blueprints/Save/MainSave` (`self.PlayerSave`)))
  (set `/Game/Blueprints/Save/MainSave.PlayerLocation` (`Actor.K2_GetActorLocation` _returnvalue) _asmain_save)
  (bind _asplayer (cast `/Game/Blueprints/Player/Player` _returnvalue))
  (set `/Game/Blueprints/Save/MainSave.PlayerCapsuleRotation` (`SceneComponent.K2_GetComponentRotation` (`Character.CapsuleComponent` _returnvalue)) _asmain_save)
  (set `/Game/Blueprints/Save/MainSave.PlayerCameraRotation` (`SceneComponent.K2_GetComponentRotation` (`/Game/Blueprints/Player/Player.Camera` _asplayer)) _asmain_save)
  (`GameplayStatics.SaveGameToSlot` _asmain_save "Save1"))

(fn `SaveWorld`
  (bind _asmain_save (cast `/Game/Blueprints/Save/MainSave` (`self.PlayerSave`)))
  (bind _outactors (`GameplayStatics.GetAllActorsOfClass` "/Game/Blueprints/World/Sky/SkyControl.SkyControl_C"))
  (set `/Game/Blueprints/Save/MainSave.WorldStruct` (make `/Game/Blueprints/Save/WorldStruct` (`TimelineComponent.GetPlaybackPosition` (`/Game/Blueprints/World/Sky/SkyControl.SkyTime` (`KismetArrayLibrary.Array_Get` _outactors)))) _asmain_save)
  (`GameplayStatics.SaveGameToSlot` _asmain_save "Save1"))