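; First-person player with movement, mouse look and a main menu on Escape or M.
; A per-tick camera line trace feeds custom-depth highlighting of "Interactive" components and right-click actions.
; Right mouse steers a BP_Boat through "Controllable" parts while locking the view, toggles sails on "Interactive" parts, or carries non-boat physics objects via a physics handle until released.
; Tick also moves the held object and eases any equipped item toward the camera.
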(event EventBeginPlay
  (Utilities|FlowControl|Sequence
    (:then_0
      ;[1 1 1] Main menu
      (bind _returnvalue (UserInterface|CreateWidget "/Game/UI/MainMenu.MainMenu_C"))
      (bind _output_get (Variables|Default|SetMainMenu _returnvalue)))))

(event EventTick
  (params (DeltaSeconds :type Float%20%28single-precision%29))
  (Utilities|FlowControl|Sequence
    (:then_0
      (bind _hit (CallFunction|Linetrace 2e+02))
      (Variables|Default|SetHitObject _hit))
    (:then_1
      (CallFunction|UpdatePickupLocation 2e+02))
    (:then_2
      (CallFunction|HoldItem "0, 0, 0" 5.0))
    (:then_3
      ;[1 1 1] Highlight interactive object
      (if (.bBlockingHit (Collision|BreakHitResult (Variables|Default|GetHitObject)))
        (if (Components|ComponentHasTag (.HitComponent (Collision|BreakHitResult (Variables|Default|GetHitObject))) "Interactive")
          (if (!= (.HitComponent (Collision|BreakHitResult (Variables|Default|GetHitObject))) (Variables|Default|GetHighlitComponent))
            (Rendering|SetRenderCustomDepth (Variables|Default|GetHighlitComponent) false)
            (Variables|Default|SetHighlitComponent (.HitComponent (Collision|BreakHitResult (Variables|Default|GetHitObject))))
            (Rendering|SetRenderCustomDepth (.HitComponent (Collision|BreakHitResult (Variables|Default|GetHitObject))) true))
          (else
            (Rendering|SetRenderCustomDepth (Variables|Default|GetHighlitComponent) false :!label _label)
            (Variables|Default|SetHighlitComponent 0)))
        (else
          (goto _label))))))

(event Input|ActionEvents|InputActionJump
  ;[1 1 1] Movement
)

(event Input|AxisEvents|InputAxisTurn
  (params (AxisValue :type Float%20%28single-precision%29))
  ;[1 1 1] Mouse look
  (Variables|Default|SetMouseX AxisValue)
  (if (not (Variables|Default|GetControlling))
    (Pawn|Input|AddControllerYawInput (|(Value*{50BE9233-4534-A410-6F3C-54B04A695433}) AxisValue))))

(event Input|AxisEvents|InputAxisMoveForwardBack
  (params (AxisValue :type Float%20%28single-precision%29))
  ;[1 1 1] Movement
  (Pawn|Input|AddMovementInput (Transformation|GetActorForwardVector) AxisValue false))

(event Input|AxisEvents|InputAxisMoveLeftRight
  (params (AxisValue :type Float%20%28single-precision%29))
  ;[1 1 1] Movement
  (Pawn|Input|AddMovementInput (Transformation|GetActorRightVector) AxisValue false))

(event Input|AxisEvents|InputAxisLookUpDown
  (params (AxisValue :type Float%20%28single-precision%29))
  ;[1 1 1] Mouse look
  (Variables|Default|SetMouseY AxisValue)
  (if (not (Variables|Default|GetControlling))
    (Pawn|Input|AddControllerPitchInput (|(Value*{50BE9233-4534-A410-6F3C-54B04A695433}) AxisValue))))

(event Input|MouseEvents|RightMouseButton
  ;[1 1 1] Pick up/drop physics objects
  (:Pressed
    (CallFunction|PickUpPhysicsObject))
  (:Released
    (CallFunction|DropPhysicsObject)))

(event Input|MouseEvents|RightMouseButton
  (bind _hitobject (Variables|Default|GetHitObject))
  (bind (_bblockinghit _binitialoverlap _time _location _impactpoint _normal _impactnormal _physmat _hitactor _hitcomponent) (Collision|BreakHitResult _hitobject))
  ;[1 1 1] Toggle object control
  (:Pressed
    (if _bblockinghit
      (if (Components|ComponentHasTag _hitcomponent "Controllable")
        (Variables|Default|SetControlling true)
        (bind _asbp_boat (Utilities|Casting|CastToBP_Boat _hitactor))
        (Variables|/Game/Blueprints/Boat/BP_Boat.BP_Boat_C|SetSteeringEnabled _asbp_boat true)
        (else
          (Variables|Default|SetControlling false)
          (bind _asbp_boat_2 (Utilities|Casting|CastToBP_Boat _hitactor :!label _label))
          (Variables|/Game/Blueprints/Boat/BP_Boat.BP_Boat_C|SetSteeringEnabled _asbp_boat_2 false)))))
  (:Released
    (Variables|Default|SetControlling false)
    (goto _label)))

(event Input|KeyboardEvents|M
  (bind _returnvalue (Game|GetPlayerController 0))
  ;[1 1 1] Main menu
  (:Pressed
    (UserInterface|Viewport|AddtoViewport (stale EventBeginPlay _output_get) 0)
    (Input|SetInputModeUIOnly _returnvalue (stale EventBeginPlay _output_get) false)
    (Variables|/Script/Engine.PlayerController|SetbShowMouseCursor _returnvalue true)))

(event Input|KeyboardEvents|Escape
  (bind _returnvalue (Game|GetPlayerController 0))
  ;[1 1 1] Main menu
  (:Pressed
    (UserInterface|Viewport|AddtoViewport (stale EventBeginPlay _output_get) 0)
    (Input|SetInputModeUIOnly _returnvalue (stale EventBeginPlay _output_get) false)
    (Variables|/Script/Engine.PlayerController|SetbShowMouseCursor _returnvalue true)))

(event Input|MouseEvents|RightMouseButton
  (bind _hitobject (Variables|Default|GetHitObject))
  (bind (_bblockinghit _binitialoverlap _time _location _impactpoint _normal _impactnormal _physmat _hitactor _hitcomponent) (Collision|BreakHitResult _hitobject))
  ;[1 1 1] Interact
  (:Pressed
    (if _bblockinghit
      (if (Components|ComponentHasTag _hitcomponent "Interactive")
        (bind _asbp_boat (Utilities|Casting|CastToBP_Boat _hitactor))
        (Default|ToggleSails _asbp_boat)))))

(fn ConstructionScript)

(fn Linetrace
  (params (Range :type Float%20%28single-precision%29))
  (bind _camera (Variables|Default|GetCamera))
  (bind _returnvalue (Transformation|GetWorldLocation _camera))
  (bind _outhit (Collision|LineTraceByChannel _returnvalue (+ _returnvalue (* (Math|Vector|GetForwardVector (Transformation|GetWorldRotation _camera)) Range)) "TraceTypeQuery1" false 0 "None"))
  (return _outhit))

(fn PickUpPhysicsObject
  (bind _hitobject (Variables|Default|GetHitObject))
  (bind (_bblockinghit _binitialoverlap _time _location _impactpoint _normal _impactnormal _physmat _hitactor _hitcomponent) (Collision|BreakHitResult _hitobject))
  (if _bblockinghit
    (if (Math|Boolean|ANDBoolean (not (Variables|Default|GetPhysicsHandleActive)) (Physics|IsSimulatingPhysics _hitcomponent "None") (!= (Utilities|GetClass _hitactor) "/Game/Blueprints/Boat/BP_Boat.BP_Boat_C"))
      (Variables|Default|SetPhysicsHandleActive true)
      (Class|PhysicsHandleComponent|GrabComponent (Variables|Default|GetPhysicsHandle) _hitcomponent "None" _location true))))

(fn DropPhysicsObject
  (if (Variables|Default|GetPhysicsHandleActive)
    (Variables|Default|SetPhysicsHandleActive false)
    (Physics|Components|PhysicsHandle|ReleaseComponent (Variables|Default|GetPhysicsHandle))))

(fn UpdatePickupLocation
  (params (Distance :type Float%20%28single-precision%29))
  (bind _camera (Variables|Default|GetCamera))
  (if (Variables|Default|GetPhysicsHandleActive)
    (Class|PhysicsHandleComponent|SetTargetLocationandRotation (Variables|Default|GetPhysicsHandle) (+ (Transformation|GetActorLocation) (* (Math|Vector|GetForwardVector _camera) Distance) "0,0,50.000000") (Transformation|GetWorldRotation _camera))))

(fn HoldItem
  (params (Offset :type Vector) (Speed :type Float%20%28single-precision%29))
  (bind _returnvalue (Utilities|Time|GetWorldDeltaSeconds))
  (bind _camera (Variables|Default|GetCamera))
  (bind _equippeditem (Variables|Default|GetEquippedItem))
  (Utilities|IsValid _equippeditem
    (:Is%20Valid
      (Transformation|SetActorLocationAndRotation _equippeditem (Math|Interpolation|VInterpTo (Transformation|GetActorLocation _equippeditem) (+ (Transformation|GetWorldLocation _camera) (Math|Vector|RotateVector Offset (Transformation|GetWorldRotation _camera))) _returnvalue Speed) (Math|Interpolation|RInterpTo (Transformation|GetActorRotation _equippeditem) (Transformation|GetWorldRotation _camera) _returnvalue Speed)))))