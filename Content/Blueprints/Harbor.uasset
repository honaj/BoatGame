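; Harbor actor that animates the brightness of a light material on its static mesh.
; On BeginPlay it creates a dynamic material instance for one mesh material slot and sets the timeline to a random start time, offsetting the animation per instance.
; The timeline's LightIntensity track drives the material's Brightness parameter on each update.
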(event `self.ReceiveBeginPlay`
  (`parent.ReceiveBeginPlay`)
  (`|ExecutionSequence`
    (:`then_0`
      (bind _returnvalue (`PrimitiveComponent.CreateDynamicMaterialInstance` (`self.StaticMeshComponent`) 8 "/Game/Materials/LightMat.LightMat"))
      (set `self.LightMat` _returnvalue))
    (:`then_1`
      (bind (_direction _lightintensity) (`Timeline|Timeline_0` :`NewTime` (`KismetMathLibrary.RandomFloatInRange` 0.0 2.0) :!via `SetNewTime`)
        (:`Update`
          (`MaterialInstanceDynamic.SetScalarParameterValue` (`self.LightMat`) "Brightness" _lightintensity))))))

(event `self.ReceiveActorBeginOverlap`
  (params (OtherActor :type "Actor Object Reference")))

(event `self.ReceiveTick`
  (params (DeltaSeconds :type "Float (single-precision)")))

(fn `UserConstructionScript`
  (`parent.UserConstructionScript`))