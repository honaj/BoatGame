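; TimeControl is a world Blueprint that animates fog over time through the FogParams material parameter collection.
; On BeginPlay it starts a slowed timeline that writes fog intensity, start distance and five colors each update.
; A FlipFlop on the timeline's finish alternates reverse and forward playback, looping it back and forth.
; Sky sphere horizon and zenith color assignments are present but disconnected, so they never run.
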(event `self.ReceiveBeginPlay`
  (`TimelineComponent.SetPlayRate` (`self.Timeline_0`) 0.2)
  (bind (_direction _intensity _startdistance _color1 _color2 _color3 _color4 _color5 _horizoncolor _zenithcolor) (`Timeline|Timeline_0` :!label _label)
    (:`Update`
      (`KismetMaterialLibrary.SetScalarParameterValue` "/Game/Materials/PostProcess/FogParams.FogParams" "Intensity" _intensity)
      (`KismetMaterialLibrary.SetScalarParameterValue` "/Game/Materials/PostProcess/FogParams.FogParams" "StartDistance" _startdistance)
      (`KismetMaterialLibrary.SetVectorParameterValue` "/Game/Materials/PostProcess/FogParams.FogParams" "Color1" _color1)
      (`KismetMaterialLibrary.SetVectorParameterValue` "/Game/Materials/PostProcess/FogParams.FogParams" "Color2" _color2)
      (`KismetMaterialLibrary.SetVectorParameterValue` "/Game/Materials/PostProcess/FogParams.FogParams" "Color3" _color3)
      (`KismetMaterialLibrary.SetVectorParameterValue` "/Game/Materials/PostProcess/FogParams.FogParams" "Color4" _color4)
      (`KismetMaterialLibrary.SetVectorParameterValue` "/Game/Materials/PostProcess/FogParams.FogParams" "Color5" _color5))
    (:`Finished`
      (`/Engine/EditorBlueprintResources/StandardMacros.FlipFlop`
        (:`A`
          (goto _label :!via `Reverse`))
        (:`B`
          (goto _label))))))

(event `self.ReceiveTick`
  (params (DeltaSeconds :type "Float (single-precision)")))

(fn `UserConstructionScript`)