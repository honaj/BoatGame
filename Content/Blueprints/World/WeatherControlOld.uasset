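; Weather controller actor that keeps a field of up to 200 randomly placed, rotated and scaled clouds high above the player.
; Each tick it samples the player location and, while below the cap, spawns one Cloud using a random stream.
; At the cap, it instead sets each cloud's material opacity by distance ratio and destroys those beyond CloudDistance, freeing slots for respawning.
; The stream seeding and an unseeded spawn variant are disconnected.
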(event EventBeginPlay)

(event EventTick
  (params (DeltaSeconds :type Float%20%28single-precision%29))
  (bind _returnvalue (|({170C74FD-4A29-719F-7EAE-7BAF2730C7F0}-({170C74FD-4A29-719F-7EAE-7BAF2730C7F0}*2))))
  (bind _cloudarray (Variables|Default|GetCloudArray))
  (bind _clouddistance (Variables|Default|GetCloudDistance))
  (bind _cloudstream (Variables|Default|GetCloudStream))
  (Utilities|FlowControl|Sequence
    (:then_0
      (Variables|Default|SetPlayerLocation (Transformation|GetActorLocation (Game|GetPlayerCharacter 0))))
    (:then_1
      (if (< (Utilities|Array|Length (Variables|Default|GetCloudArray)) 200)
        (bind _returnvalue_2 (Game|SpawnActorfromClass "/Game/Blueprints/World/Sky/Cloud.Cloud_C" (Math|Transform|MakeTransform (+ (Variables|Default|GetPlayerLocation) (Math|Vector|MakeVector (Math|Random|RandomFloatinRangefromStream _returnvalue _clouddistance _cloudstream) (Math|Random|RandomFloatinRangefromStream _returnvalue _clouddistance _cloudstream) (Math|Random|RandomFloatinRangefromStream 1.5e+05 1.7e+05 _cloudstream))) (Math|Rotator|MakeRotator 0.0 (Math|Random|RandomFloatinRangefromStream 0.0 3.6e+02 _cloudstream) (Math|Random|RandomFloatinRangefromStream 0.0 3.6e+02 _cloudstream)) (Math|Vector|MakeVector (Math|Random|RandomFloatinRangefromStream 3e+03 8e+03 _cloudstream) (Math|Random|RandomFloatinRangefromStream 3e+03 8e+03 _cloudstream) (Math|Random|RandomFloatinRangefromStream 2e+03 5e+03 _cloudstream))) true 0 0))
        (Utilities|Array|Add (Variables|Default|GetCloudArray) _returnvalue_2)
        (else
          (for _array_element _cloudarray
            (bind _returnvalue_3 (Class|ITween|GetDistanceBetweenTwoVectors (Transformation|GetActorLocation _array_element) (Variables|Default|GetPlayerLocation)))
            (Rendering|Material|SetScalarParameterValue (Variables|/Game/Blueprints/World/Sky/Cloud.Cloud_C|GetMaterial _array_element) "Opacity" (Math|Float|Clamp(Float) (/ _returnvalue_3 (Variables|Default|GetCloudDistance))) :!class /Script/Engine.MaterialInstanceDynamic)
            (if (> _returnvalue_3 (Variables|Default|GetCloudDistance))
              (Actor|DestroyActor _array_element)
              (Utilities|Array|RemoveItem _cloudarray _array_element))))))))

(fn ConstructionScript)