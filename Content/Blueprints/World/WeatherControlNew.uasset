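; Weather control Blueprint that spawns up to 200 clouds high above the player, built from a scaled-up rock mesh.
; Each Tick it caches the player location and adds one randomly placed, rotated and scaled Instanced Static Mesh component, with no instances added.
; Each cloud gets a dynamic material, stored in an array alongside its component.
; The loop for distance-based opacity and removal of distant clouds is disconnected and never runs.
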(event EventTick
  (params (DeltaSeconds :type Float%20%28single-precision%29))
  (bind _returnvalue (|({170C74FD-4A29-719F-7EAE-7BAF2730C7F0}-({170C74FD-4A29-719F-7EAE-7BAF2730C7F0}*2))))
  (bind _clouddistance (Variables|Default|GetCloudDistance))
  (Utilities|FlowControl|Sequence
    (:then_0
      (Variables|Default|SetPlayerLocation (Transformation|GetActorLocation (Game|GetPlayerCharacter 0))))
    (:then_1
      (if (< (Utilities|Array|Length (Variables|Default|GetCloudArray)) 200)
        (bind _returnvalue_2 (AddComponent|AddInstancedStaticMeshComponent false (Math|Transform|MakeTransform (+ (Variables|Default|GetPlayerLocation) (Math|Vector|MakeVector (Math|Random|RandomFloatinRange _returnvalue _clouddistance) (Math|Random|RandomFloatinRange _returnvalue _clouddistance) (Math|Random|RandomFloatinRange 1.5e+05 1.7e+05))) (Math|Rotator|MakeRotator 0.0 (Math|Random|RandomFloatinRange 0.0 3.6e+02) (Math|Random|RandomFloatinRange 0.0 3.6e+02)) (Math|Vector|MakeVector (Math|Random|RandomFloatinRange 3e+03 8e+03) (Math|Random|RandomFloatinRange 3e+03 8e+03) (Math|Random|RandomFloatinRange 2e+03 5e+03)))))
        (Components|StaticMesh|SetStaticMesh _returnvalue_2 "/Game/RealisticRocksVol1/Meshes/SmallRock01.SmallRock01")
        (bind _returnvalue_3 (Rendering|Material|CreateDynamicMaterialInstance _returnvalue_2 0 "/Game/Materials/BaseMat.BaseMat" :!class /Script/Engine.PrimitiveComponent))
        (Utilities|Array|Add (Variables|Default|GetCloudMat) _returnvalue_3)
        (Utilities|Array|Add (Variables|Default|GetCloudArray) _returnvalue_2)
        (Development|PrintString "Cloud added!")))))

(fn ConstructionScript)