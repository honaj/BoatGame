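; Day/night cycle Blueprint that animates the sun and sky over time with a slow WorldTime timeline started on BeginPlay.
; Each update pitches the Sun, refreshes the SkySphere and writes horizon color and shadow strength to the UnlitPostParamaters material parameter collection.
; A FlipFlop on Finished is wired to alternate reverse and forward playback.
; Disconnected leftovers include a second timeline for fog and sky colors, a start-time offset and direct SkySphere color assignment.
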(event `self.ReceiveBeginPlay`
  (`TimelineComponent.SetPlayRate` (`self.WorldTime`) 0.2)
  (bind (_direction _fogintensity _fogdistance _shadowstrength _sunrotation _sunbrightness _horizoncolor _zenithcolor) (`Timeline|WorldTime` :!label _label)
    (:`Update`
      (`self.SetActorRotation` (`self.Sun`) (`KismetMathLibrary.MakeRotator` _sunrotation))
      (`KismetMaterialLibrary.SetVectorParameterValue` "/Game/PostProcess/UnlitPostParamaters.UnlitPostParamaters" "SkyColorLow" _horizoncolor)
      (`/Engine/EngineSky/BP_Sky_Sphere.UpdateSunDirection` (`self.SkySphere`))
      (`KismetMaterialLibrary.SetScalarParameterValue` "/Game/PostProcess/UnlitPostParamaters.UnlitPostParamaters" "ShadowStrength" _shadowstrength))
    (:`Finished`
      (`/Engine/EditorBlueprintResources/StandardMacros.FlipFlop`
        (:`A`
          (goto _label :!via `Reverse`))
        (:`B`
          (goto _label))))))

(event `self.ReceiveTick`
  (params (DeltaSeconds :type "Float (single-precision)")))

(fn `UserConstructionScript`)