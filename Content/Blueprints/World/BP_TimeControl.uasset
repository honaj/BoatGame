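; BP_TimeControl runs the world's day-night cycle and clock through the SkyTime timeline, seeded from Time with TimeSpeed as play rate.
; Timeline updates rotate the sun and moon, set sun intensity, refresh the sky sphere, and write shadow strength and fog start to a material parameter collection.
; They also derive 24-hour, 12-hour and minute values.
; BeginPlay applies the starting time only when no "Save1" save exists.
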(event `self.ReceiveBeginPlay`
  (bind _sun (`self.Sun`))
  (`TimelineComponent.SetPlayRate` (`self.SkyTime`) (`self.TimeSpeed`))
  (bind _returnvalue (`GameplayStatics.DoesSaveGameExist` "Save1"))
  (if (not _returnvalue)
    (bind (_direction _sunpitch _sunyaw _24hourclock _12hourclock _moonpitch _moonyaw _sunintensity _shadowstrength _fogstartdistance) (`Timeline|SkyTime` :`NewTime` (`self.Time`) :!via `SetNewTime`)
      (:`Update`
        (`self.SetActorRotation` _sun (`KismetMathLibrary.MakeRotator` _sunpitch _sunyaw))
        (`LightComponent.SetIntensity` (`Light.LightComponent` _sun) _sunintensity)
        (`/Game/Blueprints/World/Sky/BP_My__Sky_Sphere.UpdateSunDirection` (`self.SkySphere`))
        (`self.SetActorRotation` (`self.MoonLight`) (`KismetMathLibrary.MakeRotator` _moonpitch _moonyaw))
        (`KismetMaterialLibrary.SetScalarParameterValue` "/Game/PostProcess/UnlitPostParamaters.UnlitPostParamaters" "ShadowStrength" _shadowstrength)
        (`KismetMaterialLibrary.SetScalarParameterValue` "/Game/PostProcess/UnlitPostParamaters.UnlitPostParamaters" "StartDistance" _fogstartdistance)
        ;[1 1 1] Time
        (set `self.Current24Hour` (`KismetMathLibrary.FFloor` _24hourclock))
        (set `self.CurrentMinute` (`KismetMathLibrary.FFloor` (`KismetMathLibrary.FMod` (* _24hourclock 60.0) 60.0)))
        (set `self.Current12Hour` (`KismetMathLibrary.FFloor` _12hourclock))))))

(event `self.ReceiveActorBeginOverlap`
  (params (OtherActor :type "Actor Object Reference")))

(event `self.ReceiveTick`
  (params (DeltaSeconds :type "Float (single-precision)")))

(fn `UserConstructionScript`
  (`TimelineComponent.SetNewTime` (`self.SkyTime`) (`KismetMathLibrary.FClamp` (`self.Time`) 0.0 24.0))
  (`TimelineComponent.SetPlayRate` (`self.SkyTime`) (`self.TimeSpeed`)))