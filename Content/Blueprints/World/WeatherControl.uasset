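; WeatherControl keeps a field of up to 200 cloud actors in the sky around the player.
; Each tick it spawns one cloud high above the player with random offset, rotation and scale until the array is full.
; Once full, it instead sets each cloud's material opacity from its player distance relative to CloudDistance, more opaque when farther.
; Clouds beyond that distance are destroyed and removed, letting spawning refill the array.
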(event EventTick
  (params (DeltaSeconds :type Float%20%28single-precision%29))
  (bind _returnvalue (|({170C74FD-4A29-719F-7EAE-7BAF2730C7F0}-({170C74FD-4A29-719F-7EAE-7BAF2730C7F0}*2))))
  (bind _clouddistance (Variables|Default|GetCloudDistance))
  (bind _cloudarray (Variables|Default|GetCloudArray))
  (Utilities|FlowControl|Sequence
    (:then_0
      (Variables|Default|SetPlayerLocation (Transformation|GetActorLocation (Game|GetPlayerCharacter 0))))
    (:then_1
      (if (< (Utilities|Array|Length (Variables|Default|GetCloudArray)) 200)
        (bind _returnvalue_2 (Game|SpawnActorfromClass "/Game/Blueprints/World/Cloud.Cloud_C" (Math|Transform|MakeTransform (+ (Transformation|GetActorLocation (Game|GetPlayerCharacter 0)) (Math|Vector|MakeVector (Math|Random|RandomFloatinRange _returnvalue _clouddistance) (Math|Random|RandomFloatinRange _returnvalue _clouddistance) (Math|Random|RandomFloatinRange 1.5e+05 1.7e+05))) (Math|Rotator|MakeRotator 0.0 (Math|Random|RandomFloatinRange 0.0 3.6e+02) (Math|Random|RandomFloatinRange 0.0 3.6e+02)) (Math|Vector|MakeVector (Math|Random|RandomFloatinRange 3e+03 8e+03) (Math|Random|RandomFloatinRange 3e+03 8e+03) (Math|Random|RandomFloatinRange 2e+03 5e+03))) true 0 0))
        (Utilities|Array|Add (Variables|Default|GetCloudArray) _returnvalue_2)
        (Development|PrintString "Cloud added!")
        (else
          (for _array_element _cloudarray
            (bind _returnvalue_3 (Class|ITween|GetDistanceBetweenTwoVectors (Transformation|GetActorLocation _array_element) (Variables|Default|GetPlayerLocation)))
            (Rendering|Material|SetScalarParameterValue (Variables|/Game/Blueprints/World/Cloud.Cloud_C|GetMaterial _array_element) "Opacity" (Math|Float|Clamp(Float) (/ _returnvalue_3 (Variables|Default|GetCloudDistance))) :!class /Script/Engine.MaterialInstanceDynamic)
            (if (> _returnvalue_3 (Variables|Default|GetCloudDistance))
              (Actor|DestroyActor _array_element)
              (Utilities|Array|RemoveItem _cloudarray _array_element)
              (Development|PrintString "Cloud deleted!"))))))))

(fn ConstructionScript)